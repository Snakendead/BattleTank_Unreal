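; Player-controllable tank pawn Blueprint that wires input to its aiming and movement components.
; On BeginPlay it hands the barrel and turret to TankAiming and the left and right tracks to TankMovement.
; Aim axes rotate a camera rig, with yaw on the azimuth gimbal and pitch on the spring arm.
; Move and turn axes send intents to TankMovement, and the Fire action calls TankAiming.Fire.
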(event `self.ReceiveBeginPlay`
  (`TankAimingComponent.Initialize` (`self.TankAiming`) (`self.Barrel`) (`self.Turret`))
  (`TankMovementComponent.Initialize` (`self.TankMovement`) (`self.Left Track`) (`self.Rigth Track`)))

(event `InputAxis|AimElevation`
  (params (AxisValue :type "Float (single-precision)"))
  ;[1 1 1] Aim Input Control
  (`SceneComponent.K2_AddLocalRotation` (`self.SpringArm`) (`KismetMathLibrary.MakeRotator` 0.0 AxisValue) false false))

(event `InputAxis|AimAzimuth`
  (params (AxisValue :type "Float (single-precision)"))
  ;[1 1 1] Aim Input Control
  (`SceneComponent.K2_AddLocalRotation` (`self.AzimuthGimbal`) (`KismetMathLibrary.MakeRotator` 0.0 0.0 AxisValue) false false))

(event `InputAxis|Move Forward`
  (params (AxisValue :type "Float (single-precision)"))
  ;[1 1 1] Move control
  (`TankMovementComponent.IntendMoveForward` (`self.TankMovement`) AxisValue))

(event `InputAction|Fire`
  (params (Key :type "Key Structure"))
  ;[1 1 1] Aim Input Control
  (:`Pressed`
    (`TankAimingComponent.Fire` (`self.TankAiming`))))

(event `InputAxis|Turn Right`
  (params (AxisValue :type "Float (single-precision)"))
  ;[1 1 1] Move control
  (`TankMovementComponent.IntendTurnRight` (`self.TankMovement`) AxisValue))

(fn `UserConstructionScript`)